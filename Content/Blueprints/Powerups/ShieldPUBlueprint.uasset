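; Shield powerup Blueprint that absorbs incoming damage for the player cube it attaches to.
; On attach it saves the cube visual's material and swaps in a shield material, then restores the original on detach.
; OnTakeDamage subtracts damage from the shield capacity and returns only the overflow once it reaches zero or below, otherwise zero.
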(event EventOnAttach
  (params (PlayerCube :type Player%20Cube%20Object%20Reference))
  (bind _cubevisual (Variables|/Script/CubeWars.PlayerCube|GetCubeVisual PlayerCube))
  (|CallParentFunction PlayerCube)
  (Variables|Default|SetOldMaterial (Rendering|Material|GetMaterial _cubevisual 0))
  (Rendering|Material|SetMaterial _cubevisual 0 (Variables|Default|GetNewMaterial)))

(event EventOnDetach
  (bind _returnvalue (Class|PowerUp|GetPlayerCube))
  (Rendering|Material|SetMaterial (Variables|/Script/CubeWars.PlayerCube|GetCubeVisual _returnvalue) 0 (Variables|Default|GetOldMaterial))
  (|CallParentFunction))

(fn OnTakeDamage
  (params (DamageAmount :type Float%20%28single-precision%29) (DamageEvent :type Damage%20Event%20Structure%20%28by%20ref%29) (EventInstigator :type Controller%20Object%20Reference) (DamageCauser :type Actor%20Object%20Reference))
  (bind _output_get (Variables|Default|SetShieldCapacity (- (Variables|Default|GetShieldCapacity) DamageAmount)))
  (if (<= _output_get 0.0)
    (return (Math|Float|Absolute(Float) _output_get))
    (else
      (return 0.0))))

(fn ConstructionScript)