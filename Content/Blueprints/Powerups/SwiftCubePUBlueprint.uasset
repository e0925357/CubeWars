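; Swift cube powerup that changes the player cube's movement speed while it is attached.
; On attach it runs the parent logic, saves the cube's current CubeMovement speed as OldSpeed, then applies NewSpeed.
; On detach it restores OldSpeed before handing off to the parent detach logic.
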(event EventOnAttach
  (params (PlayerCube :type Player%20Cube%20Object%20Reference))
  (bind _cubemovement (Variables|/Script/CubeWars.PlayerCube|GetCubeMovement PlayerCube))
  (|CallParentFunction PlayerCube)
  (bind _returnvalue (Class|PlayerCubeMovementComponent|GetSpeed _cubemovement))
  (Variables|Default|SetOldSpeed _returnvalue)
  (Class|PlayerCubeMovementComponent|SetSpeed _cubemovement (Variables|Default|GetNewSpeed)))

(event EventOnDetach
  (bind _returnvalue (Class|PowerUp|GetPlayerCube))
  (Class|PlayerCubeMovementComponent|SetSpeed (Variables|/Script/CubeWars.PlayerCube|GetCubeMovement _returnvalue) (Variables|Default|GetOldSpeed))
  (|CallParentFunction))

(fn ConstructionScript)