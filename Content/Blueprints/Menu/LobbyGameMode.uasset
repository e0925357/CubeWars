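; Lobby game mode that relays player join and leave events to the Lobby object held in LobbyWidget.
; PostLogin calls OnNewPlayer only when the player count equals two, while OnLogout calls OnPlayerLeft without checking the count.
; Both paths depend on a successful cast of LobbyWidget, which this graph never assigns.
; BeginPlay, Tick and the construction script are empty, and a leftover one-player count check is unconnected.
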(event EventBeginPlay)

(event EventTick
  (params (DeltaSeconds :type Float%20%28single-precision%29)))

(event EventPostLogin
  (params (NewPlayer :type Player%20Controller%20Object%20Reference))
  (bind _aslobby (Utilities|Casting|CastToLobby (Variables|Components|GetLobbyWidget)))
  (bind _returnvalue (Class|GameMode|GetNumPlayers))
  (if (== _returnvalue 2)
    (Default|OnNewPlayer _aslobby)))

(event EventOnLogout
  (params (ExitingController :type Controller%20Object%20Reference))
  (bind _aslobby (Utilities|Casting|CastToLobby (Variables|Components|GetLobbyWidget)))
  (Default|OnPlayerLeft _aslobby))

(fn ConstructionScript)