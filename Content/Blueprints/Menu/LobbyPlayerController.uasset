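; Player controller for the multiplayer lobby menu that sends the local player's name and relays lobby names to the HUD.
; On BeginPlay it shows the cursor, enables click events and HUD input, then, for the local controller, reads the name from CubeGameInstance and passes it to SetPlayerNameBP.
; OnUpdatePlayerNames forwards both player names to LobbyHUD for display.
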(event EventOnUpdatePlayerNames
  (params (Player1Name :type String) (Player2Name :type String))
  (bind _aslobby_hud (Utilities|Casting|CastToLobbyHUD (HUD|GetHUD)))
  (Default|UpdatePlayerNames _aslobby_hud Player1Name Player2Name))

(event EventBeginPlay
  ;[1 1 1] Sets the player name
  (Variables|Default|SetbEnableClickEvents true)
  (Variables|Default|SetbShowMouseCursor true)
  (Input|EnableInput (HUD|GetHUD) self)
  (if (Pawn|IsLocalPlayerController)
    (bind _ascube_game_instance (Utilities|Casting|CastToCubeGameInstance (Game|GetGameInstance)))
    (bind _returnvalue (Class|CubeGameInstance|GetPlayerName _ascube_game_instance))
    (Class|NamedPlayerController|SetPlayerNameBP _returnvalue)))

(event EventTick
  (params (DeltaSeconds :type Float%20%28single-precision%29)))

(fn ConstructionScript)