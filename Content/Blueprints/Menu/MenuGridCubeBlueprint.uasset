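; A menu grid cube Blueprint that takes a random color from its Colors array on BeginPlay.
; It creates dynamic material instances for the VisualRepresentation and Trail components, then applies the color to both through SetCubeColor.
; The glow color is derived from the chosen color via HSV, keeping hue and value but fixing a low saturation for a paler tint.
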(event EventBeginPlay
  (bind _trail (Variables|Default|GetTrail))
  (bind _colors (Variables|Default|GetColors))
  (bind _visualrepresentation (Variables|Default|GetVisualRepresentation))
  (bind _returnvalue (Rendering|Material|CreateDynamicMaterialInstance _visualrepresentation 0 0 :!class /Script/Engine.PrimitiveComponent))
  (Rendering|Material|SetMaterial _visualrepresentation 0 _returnvalue)
  (Variables|Default|SetDynamicMaterial _returnvalue)
  (bind _returnvalue_2 (Rendering|Material|CreateDynamicMaterialInstance _trail 0 0 :!class /Script/Engine.PrimitiveComponent))
  (Rendering|Material|SetMaterial _trail 0 _returnvalue_2)
  (Variables|Default|SetDynamicTrailMat _returnvalue_2)
  (CallFunction|SetCubeColor (Utilities|Array|Get(acopy) _colors (Math|Random|RandomIntegerinRange 0 (- (Utilities|Array|Length _colors) 1)))))

(event EventActorBeginOverlap
  (params (OtherActor :type Actor%20Object%20Reference)))

(event EventTick
  (params (DeltaSeconds :type Float%20%28single-precision%29)))

(fn ConstructionScript)

(fn SetCubeColor
  (params (Color :type Linear%20Color%20Structure))
  (bind (_h _s _v) (Math|Color|RGBtoHSV(LinearColor) Color))
  (bind _dynamicmaterial (Variables|Default|GetDynamicMaterial))
  (Rendering|Material|SetVectorParameterValue _dynamicmaterial "Base Color" Color :!class /Script/Engine.MaterialInstanceDynamic)
  (Rendering|Material|SetVectorParameterValue _dynamicmaterial "Glow Color" (Class|KismetMathLibrary|HSVtoRGB _h 0.3 _v 1.0) :!class /Script/Engine.MaterialInstanceDynamic)
  (Rendering|Material|SetVectorParameterValue (Variables|Default|GetDynamicTrailMat) "BaseColor" Color :!class /Script/Engine.MaterialInstanceDynamic))