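; Player cube pawn Blueprint that pushes its health to the battle HUD.
; On HealthChanged it sets the BattleInterface health progress to Health divided by its hardcoded maximum.
; The interface reference is fetched lazily from the player controller's GameHUD when not yet valid, then reused on later changes.
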(event EventHealthChanged
  (if (Utilities|IsValid (Variables|Default|GetBattleInterface))
    (Default|SetHealthProgress (Variables|Default|GetBattleInterface) (/ (Variables|Default|GetHealth) 1e+02) :!label _label)
    (else
      (bind _asplayer_controller (Utilities|Casting|CastToPlayerController (Pawn|GetController)))
      (bind _asgame_hud (Utilities|Casting|CastToGameHUD (HUD|GetHUD _asplayer_controller)))
      (Variables|Default|SetBattleInterface (Variables|/Game/Blueprints/GameHUD.GameHUD_C|GetBattleInterface _asgame_hud))
      (if (Utilities|IsValid (Variables|Default|GetBattleInterface))
        (goto _label)))))

(event EventBeginPlay)

(event Collision|EventActorBeginOverlap
  (params (OtherActor :type Actor%20Object%20Reference)))

(event EventTick
  (params (DeltaSeconds :type Float%20%28single-precision%29)))

(fn ConstructionScript)