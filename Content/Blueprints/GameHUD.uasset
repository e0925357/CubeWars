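; GameHUD creates and switches the match UI: a battle interface, a music display and an end-of-match screen.
; On BeginPlay it creates all three widgets but adds only the battle interface and music display to the viewport.
; GameEnded swaps the battle interface for the end screen, passes it both players' names, points and the win flag, and resets battle health progress.
; OnRematchRequest forwards to the end screen if it is valid.
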(event EventBeginPlay
  (bind _returnvalue (UserInterface|CreateWidget "/Game/UI/BattleInterface.BattleInterface_C"))
  (bind _output_get (Variables|Default|SetBattleInterface _returnvalue))
  (UserInterface|Viewport|AddtoViewport _output_get 0)
  (bind _returnvalue_2 (UserInterface|CreateWidget "/Game/UI/MatchEndedWidget.MatchEndedWidget_C"))
  (Variables|Default|SetEndGameInterface _returnvalue_2)
  (bind _returnvalue_3 (UserInterface|CreateWidget "/Game/UI/MusicDisplay.MusicDisplay_C"))
  (bind _output_get_2 (Variables|Default|SetMusicDisplay _returnvalue_3))
  (UserInterface|Viewport|AddtoViewport _output_get_2 0))

(event Collision|EventActorBeginOverlap
  (params (OtherActor :type Actor%20Object%20Reference)))

(event EventTick
  (params (DeltaSeconds :type Float%20%28single-precision%29)))

(fn ConstructionScript)

(fn GameEnded
  (params (Player1Name :type String%20%28by%20ref%29) (Player2Name :type String%20%28by%20ref%29) (Player1Points :type Integer) (Player2Points :type Integer) (HasWon :type Boolean))
  (bind _battleinterface (Variables|Default|GetBattleInterface))
  (bind _endgameinterface (Variables|Default|GetEndGameInterface))
  (Widget|RemovefromParent _battleinterface)
  (UserInterface|Viewport|AddtoViewport _endgameinterface 1)
  (Default|UpdateValues _endgameinterface Player1Name Player2Name Player1Points Player2Points HasWon)
  (Default|SetHealthProgress _battleinterface 1.0))

(fn OnRematchRequest
  (bind _endgameinterface (Variables|Default|GetEndGameInterface))
  (if (Utilities|IsValid _endgameinterface)
    (Default|OnRematchRequest _endgameinterface)))