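; BackgroundCubeSpawner is an actor that repeatedly spawns BackgroundBattlefieldCube actors as moving background scenery.
; It spawns one cube at its own transform on BeginPlay, passing Speed as the initial speed and SpawnLifeSpan as the fly time.
; Tick accumulates a timer and loops back into the same spawn chain, resetting the timer, whenever SpawnInterval elapses.
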(event EventBeginPlay
  (bind _returnvalue (Game|SpawnActorfromClass "/Game/Blueprints/Background/BackgroundBattlefieldCUbe.BackgroundBattlefieldCube_C" (Transformation|GetActorTransform) "Undefined" 0 (Variables|Default|GetSpeed) 0))
  (Default|SetFlyTime _returnvalue (Variables|Default|GetSpawnLifeSpan))
  (Variables|Default|Settimer 0.0))

(event EventTick
  (params (DeltaSeconds :type Float%20%28single-precision%29))
  (bind _output_get (Variables|Default|Settimer (+ DeltaSeconds (Variables|Default|Gettimer))))
  (if (>= _output_get (Variables|Default|GetSpawnInterval))
    (bind _returnvalue (Game|SpawnActorfromClass "/Game/Blueprints/Background/BackgroundBattlefieldCUbe.BackgroundBattlefieldCube_C" (Transformation|GetActorTransform) "Undefined" 0 (Variables|Default|GetSpeed) 0))
    (Default|SetFlyTime _returnvalue (Variables|Default|GetSpawnLifeSpan))
    (Variables|Default|Settimer 0.0)))

(fn ConstructionScript)